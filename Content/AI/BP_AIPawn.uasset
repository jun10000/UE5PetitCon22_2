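; AI pawn that provides a look-ahead target along a route spline and a ride attachment point.
; On BeginPlay it caches the first BP_AIManageActor in the level as its route actor, logging an error if none is found.
; GetTargetTransform projects the pawn's location onto that actor's spline and samples the transform ForwardDistance further along.
; GetRidePointTransform returns the world transform of the mesh's RidePoint socket.
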(event `self.ReceiveBeginPlay`
  (bind _outactors (`GameplayStatics.GetAllActorsOfClass` "/Game/AI/BP_AIManageActor.BP_AIManageActor_C"))
  (bind _output (`|GetArrayItem` _outactors))
  (`/Engine/EditorBlueprintResources/StandardMacros.IsValid` _output
    (:`Is Valid`
      (set `self.CurrentAIRouteActor` _output))
    (:`Is Not Valid`
      (`/Game/Blueprints/BP_FunctionLibrary.PrintError` "AIRouteActor not found"))))

(fn `GetRidePointTransform`
  (returns (ReturnValue :type "Transform Structure"))
  (return (`SceneComponent.GetSocketTransform` (`self.Mesh`) "RidePoint" "RTS_World")))

(fn `GetTargetTransform`
  (returns (ReturnValue :type "Transform Structure"))
  (bind _spline (`/Game/AI/BP_AIManageActor.Spline` (`self.CurrentAIRouteActor`)))
  (return (`/Game/Blueprints/BP_FunctionLibrary.GetTransformAtDistanceAlongSpline2` _spline (+ (`SplineComponent.GetDistanceAlongSplineAtLocation` _spline (`self.K2_GetActorLocation`) "World") (`self.ForwardDistance`)) "World" true)))

(fn `UserConstructionScript`)
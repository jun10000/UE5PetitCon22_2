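; AI route actor that holds a Targets list of actors, presumably the points of a route.
; GetTargetActorByIndex bounds-checks the index and returns the matching target, or prints an error and returns nothing when it is out of range.
; The actor is passive: its construction script is empty and its BeginPlay, overlap and Tick events are unused placeholders.
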(fn `GetTargetActorByIndex`
  (params (Index :type Integer))
  (returns (ReturnValue :type "Actor Object Reference"))
  (if (and (>= Index 0) (< Index (`KismetArrayLibrary.Array_Length` (`self.Targets`))))
    (return (`|GetArrayItem` (`self.Targets`) Index))
    (else
      (`/Game/Blueprints/BP_FunctionLibrary.PrintError` "AIRouteActor: Failed to get target actor")
      (return null))))

(fn `UserConstructionScript`)
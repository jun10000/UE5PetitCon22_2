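; BP_AIManageActor is a manager actor that lays out BP_AIPawn instances along its spline.
; PlaceAIPawns destroys every existing BP_AIPawn, then spawns the configured count at even spacing derived from spline length, passing each its index.
; The first pawn receives a tag read from the DT_ConstCollection data table.
; BeginPlay, Tick and the construction script are empty, so placement runs only when that event is called.
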(event `PlaceAIPawns`
  ;[1 1 1] CurrentAIPawnSpacing設定
  (set `self.CurrentAIPawnSpacing` (/ (`SplineComponent.GetSplineLength` (`self.Spline`)) (`self.PlaceAIPawnNum`)))
  ;[1 1 1] 既存のAIPawnを全削除
  (bind _outactors (`GameplayStatics.GetAllActorsOfClass` "/Game/AI/BP_AIPawn.BP_AIPawn_C"))
  (for _array_element _outactors
    (`self.K2_DestroyActor` _array_element))
  ;[1 1 1] AIPawnの自動配置
  (for _index (range (`self.PlaceAIPawnNum`))
    (bind _returnvalue (`|SpawnActorFromClass` "/Game/AI/BP_AIPawn.BP_AIPawn_C" (`/Game/Blueprints/BP_FunctionLibrary.GetTransformAtDistanceAlongSpline2` (`self.Spline`) (* _index (`self.CurrentAIPawnSpacing`)) "World" true) "Undefined" "MultiplyWithRoot" null _index null))
    ;[1 1 1] 最初のAIPawnにStartタグを追加
    (if (== _index 0)
      (bind _returnvalue_2 (`|GetDataTableRow` "/Game/Blueprints/DataTable/DT_ConstCollection.DT_ConstCollection" "Default")
        (:`then`
          (`KismetArrayLibrary.Array_Add` (`Actor.Tags` _returnvalue) (break `/Game/Blueprints/Structs/ST_ConstCollection` _returnvalue_2)))))))

(fn `UserConstructionScript`)
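; Player pawn that rides AI horse pawns and jumps between them to score points.
; Tick snaps it to the current horse's ride point with clamped pitch, starting from a horse found by a data table tag.
; A timeline swings the aiming arrow while resumed; Pause hides and stops it.
; TryJumping box-traces along the arrow, switches to the hit horse, awards distance-based points and pitches the jump sound by distance.
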(event `self.ReceiveBeginPlay`
  (`self.InitCurrentRidingHorse`)
  (`SceneComponent.K2_SetRelativeRotation` (`self.ArrowAxis`) (`KismetMathLibrary.MakeRotator` 0.0 0.0 (* (`self.ArrowRotationHalfDegree`) -1.0)) false false))

(event `Resume`
  (`SceneComponent.SetVisibility` (`self.SM_Arrow`) true false)
  (bind (_direction _zdiffratio) (`Timeline|TL_RotateArrow` :!label _label)
    (:`Update`
      (`SceneComponent.K2_SetRelativeRotation` (`self.ArrowAxis`) (`KismetMathLibrary.MakeRotator` 0.0 0.0 (* _zdiffratio (`self.ArrowRotationHalfDegree`))) false false))))

(event `Pause`
  (`SceneComponent.SetVisibility` (`self.SM_Arrow`) false false)
  (goto _label :!via `Stop`))

(event `self.ReceiveTick`
  (params (DeltaSeconds :type "Float (single-precision)"))
  (bind _currentridinghorse (`self.CurrentRidingHorse`))
  (bind _returnvalue (`/Game/AI/BP_AIPawn.GetRidePointTransform` _currentridinghorse))
  (`/Engine/EditorBlueprintResources/StandardMacros.IsValid` _currentridinghorse
    (:`Is Valid`
      (`self.K2_SetActorTransform` (`KismetMathLibrary.MakeTransform` (.location _returnvalue) (`KismetMathLibrary.MakeRotator` (.roll (.rotation _returnvalue)) (`KismetMathLibrary.ClampAngle` (.pitch (.rotation _returnvalue)) (`self.RotationYMinDegrees`) (`self.RotationYMaxDegrees`)) (.yaw (.rotation _returnvalue))) (.scale _returnvalue))))))

(fn `InitCurrentRidingHorse`
  (bind _returnvalue (`|GetDataTableRow` "/Game/Blueprints/DataTable/DT_ConstCollection.DT_ConstCollection" "Default")
    (:`then`
      (bind _outactors (`GameplayStatics.GetAllActorsOfClassWithTag` "/Game/AI/BP_AIPawn.BP_AIPawn_C" (break `/Game/Blueprints/Structs/ST_ConstCollection` _returnvalue)))
      (bind _output (`|GetArrayItem` _outactors))
      (`/Engine/EditorBlueprintResources/StandardMacros.IsValid` _output
        (:`Is Valid`
          (set `self.CurrentRidingHorse` _output))
        (:`Is Not Valid`
          (`/Game/Blueprints/BP_FunctionLibrary.PrintError` "First horse pawn not found"))))
    (:`RowNotFound`
      (`/Game/Blueprints/BP_FunctionLibrary.PrintError` "First horse pawn's tag not found"))))

(fn `TryJumping`
  (returns (IsSuccess :type Boolean))
  (bind _sm_arrow (`self.SM_Arrow`))
  (bind _returnvalue (`SceneComponent.K2_GetComponentLocation` _sm_arrow))
  (bind _outhit (`KismetSystemLibrary.BoxTraceSingle` _returnvalue (+ _returnvalue (* (`SceneComponent.GetForwardVector` _sm_arrow) (`self.TraceDistance`))) (`KismetMathLibrary.MakeVector` 0.0 0.0 (`self.TraceBoxHeightHalf`)) (struct) "TraceTypeQuery3" false (`|MakeArray` (`self.CurrentRidingHorse`) :!type "Actor Object Reference") "ForDuration" true (struct :`R` 1.0 :`A` 1.0) (struct :`G` 1.0 :`A` 1.0) 0.5))
  (bind (_asbp_aipawn _bsuccess) (cast `/Game/AI/BP_AIPawn` (`.HitActor` (`GameplayStatics.BreakHitResult` _outhit)) :!pure true))
  (if _bsuccess
    (bind _returnvalue_2 (`KismetMathLibrary.VSize` (- (`self.K2_GetActorLocation` _asbp_aipawn) (`self.K2_GetActorLocation` (`self.CurrentRidingHorse`)))))
    (`/Game/Blueprints/BP_GameMode.AddPoints` (`/Game/Blueprints/BP_FunctionLibrary.GetMyGameMode`) _returnvalue_2)
    (`GameplayStatics.PlaySound2D` "/Game/Sounds/SC_Jump.SC_Jump" 1.0 (/ (`self.JumpSoundBaseDistance`) _returnvalue_2) 0.0 null null)
    (set `self.CurrentRidingHorse` _asbp_aipawn)
    (return true)
    (else
      (return false))))

(fn `UserConstructionScript`)
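; BP_GameMode runs a timed, scored round from countdown through play to results.
; On BeginPlay it pauses the player and shows W_Countdown, whose OnGoShow event resumes play, adds W_HUD and starts BPTimerComponent with the time limit.
; When the timer finishes, it pauses again, swaps the HUD for W_Result and switches to UI-only input.
; SetPauseState toggles controller input and the pawn's Pause/Resume, while AddPoints and GetPoints manage the score.
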(event `self.ReceiveBeginPlay`
  (bind _returnvalue (`GameplayStatics.GetPlayerController` 0))
  (`self.SetPauseState` true)
  (`WidgetBlueprintLibrary.SetInputMode_GameOnly` _returnvalue)
  (set `PlayerController.bShowMouseCursor` false _returnvalue)
  (bind _returnvalue_2 (`|CreateWidget` "/Game/Widgets/W_Countdown.W_Countdown_C"))
  (add `/Game/Widgets/W_Countdown.OnGoShow` _returnvalue_2 (delegate `Event_OnGoShow`))
  (`UserWidget.AddToViewport` _returnvalue_2 0))

(event `Event_OnGoShow`
  (bind _bp_timercomponent (`self.BP_TimerComponent`))
  (`self.SetPauseState` false)
  (bind _returnvalue (`|CreateWidget` "/Game/Widgets/W_HUD.W_HUD_C"))
  (bind _output_get (set `self.CurrentHUD` _returnvalue))
  (`UserWidget.AddToViewport` _output_get 0)
  (add `/Game/Blueprints/BP_TimerComponent.OnTimerFinished` _bp_timercomponent (delegate `Event_OnTimerFinished`))
  (`/Game/Blueprints/BP_TimerComponent.StartTimer` _bp_timercomponent (`KismetMathLibrary.FromSeconds` (`self.LimitSeconds`))))

(event `Event_OnTimerFinished`
  (bind _returnvalue (`GameplayStatics.GetPlayerController` 0))
  (`self.SetPauseState` true)
  (`Widget.RemoveFromParent` (`self.CurrentHUD`))
  (bind _returnvalue_2 (`|CreateWidget` "/Game/Widgets/W_Result.W_Result_C"))
  (`UserWidget.AddToViewport` _returnvalue_2 0)
  (`WidgetBlueprintLibrary.SetInputMode_UIOnlyEx` _returnvalue null)
  (set `PlayerController.bShowMouseCursor` true _returnvalue))

(fn `AddPoints`
  (params (Points :type "Float (double-precision)"))
  (returns (Result :type "Float (double-precision)"))
  (bind _output_get (set `self.Points` (+ (`self.Points`) Points)))
  (return _output_get))

(fn `GetPoints`
  (returns (ReturnValue :type "Float (double-precision)"))
  (return (`self.Points`)))

(fn `SetPauseState`
  (params (IsPause :type Boolean))
  (bind _returnvalue (`GameplayStatics.GetPlayerController` 0))
  (bind _asbp_player_pawn (cast `/Game/Blueprints/BP_PlayerPawn` (`GameplayStatics.GetPlayerPawn` 0) :!pure true))
  (if IsPause
    (`self.DisableInput` _returnvalue null)
    (`/Game/Blueprints/BP_PlayerPawn.Pause` _asbp_player_pawn)
    (else
      (`self.EnableInput` _returnvalue null)
      (`/Game/Blueprints/BP_PlayerPawn.Resume` _asbp_player_pawn))))

(fn `UserConstructionScript`)
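; Player controller Blueprint that binds Enhanced Input actions for jumping and quitting the game.
; On BeginPlay it adds the default input mapping context to the local player's Enhanced Input subsystem.
; The jump action casts the controlled pawn to BP_PlayerPawn, calls its TryJumping and prints a success or failure message.
; The exit action quits the game.
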(event `self.ReceiveBeginPlay`
  (`EnhancedInputSubsystemInterface.AddMappingContext` (subsystem `EnhancedInputLocalPlayerSubsystem`) "/Game/Inputs/IMC_Default.IMC_Default" 0 (struct)))

(event `EnhancedInput|/Game/Inputs/IA_Jump`
  (params (ActionValue :type Boolean) (ElapsedSeconds :type "Float (double-precision)") (TriggeredSeconds :type "Float (double-precision)") (InputAction :type "InputAction Object Reference" :default "/Game/Inputs/IA_Jump.IA_Jump"))
  (:`Started`
    (bind _asbp_player_pawn (cast `/Game/Blueprints/BP_PlayerPawn` (`self.K2_GetPawn`)))
    (bind _issuccess (`/Game/Blueprints/BP_PlayerPawn.TryJumping` _asbp_player_pawn))
    (if _issuccess
      (`KismetSystemLibrary.PrintString` "成功！")
      (else
        (`KismetSystemLibrary.PrintString` "失敗")))))

(event `EnhancedInput|/Game/Inputs/IA_Exit`
  (params (ActionValue :type Boolean) (ElapsedSeconds :type "Float (double-precision)") (TriggeredSeconds :type "Float (double-precision)") (InputAction :type "InputAction Object Reference" :default "/Game/Inputs/IA_Exit.IA_Exit"))
  (:`Started`
    (`KismetSystemLibrary.QuitGame` null "Quit")))

(fn `UserConstructionScript`)
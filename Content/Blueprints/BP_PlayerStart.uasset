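; BP_PlayerStart is a player start that can be placed at the ride point of a chosen AI pawn.
; Its UpdateTransform event finds the BP_AIPawn matching UpdateTransformIndex through GetAIPawnByIndex, which searches all such actors by PawnIndex.
; It then copies that ride point's transform, shifting the location by UpdateTransformLocalOffset rotated into the ride point's orientation.
; BeginPlay and Tick are empty, so the transform changes only when UpdateTransform is invoked.
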(event `UpdateTransform`
  (bind (_returnvalue_location _returnvalue_rotation _returnvalue_scale) (`KismetMathLibrary.BreakTransform` (`/Game/AI/BP_AIPawn.GetRidePointTransform` (`self.GetAIPawnByIndex` (`self.UpdateTransform_Index`)))))
  (`self.K2_SetActorTransform` (`KismetMathLibrary.MakeTransform` (+ _returnvalue_location (`KismetMathLibrary.GreaterGreater_VectorRotator` (`self.UpdateTransform_LocalOffset`) _returnvalue_rotation)) _returnvalue_rotation _returnvalue_scale)))

(fn `GetAIPawnByIndex`
  (params (Index :type Integer))
  (returns (ReturnValue :type "/Game/AI/BP_AIPawn Object Reference"))
  (locals (CurrentReturnValue :type "/Game/AI/BP_AIPawn Object Reference"))
  (bind _outactors (`GameplayStatics.GetAllActorsOfClass` "/Game/AI/BP_AIPawn.BP_AIPawn_C"))
  (for _array_element _outactors
    (if (== (`/Game/AI/BP_AIPawn.PawnIndex` _array_element) Index)
      (set `local.CurrentReturnValue` _array_element)
      (break)))
  (return (`local.CurrentReturnValue`)))

(fn `UserConstructionScript`)